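; BP_Player is the player actor for a flipbook-sprite game, moved in four directions on the XZ plane.
; BeginPlay adds the IMC_Main Enhanced Input context, and each move action swaps the directional flipbook and offsets the location by a fixed, unswept step.
; Tick sphere-traces a short distance along the forward vector and prints the hit actor's name.
; An idle flipbook switch exists but is not connected.
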(event `self.ReceiveBeginPlay`
  (`EnhancedInputSubsystemInterface.AddMappingContext` (pcsubsystem `EnhancedInputLocalPlayerSubsystem` (`GameplayStatics.GetPlayerController` 0)) "/Game/Input/IMC_Main.IMC_Main" 0 (struct)))

(event `EnhancedInput|/Game/Input/IA_MoveDown`
  (params (ActionValue :type Boolean) (ElapsedSeconds :type "Float (double-precision)") (TriggeredSeconds :type "Float (double-precision)") (InputAction :type "InputAction Object Reference" :default "/Game/Input/IA_MoveDown.IA_MoveDown"))
  (:`Triggered`
    (`PaperFlipbookComponent.SetFlipbook` (`self.Sprite`) "/Game/Assets/PlayerTextures/16x16/FB_MoveD.FB_MoveD")
    (`self.K2_SetActorLocation` (+ (`self.K2_GetActorLocation`) (0.0 0.0 -2.0)))))

(event `EnhancedInput|/Game/Input/IA_MoveLeft`
  (params (ActionValue :type Boolean) (ElapsedSeconds :type "Float (double-precision)") (TriggeredSeconds :type "Float (double-precision)") (InputAction :type "InputAction Object Reference" :default "/Game/Input/IA_MoveLeft.IA_MoveLeft"))
  (:`Triggered`
    (`PaperFlipbookComponent.SetFlipbook` (`self.Sprite`) "/Game/Assets/PlayerTextures/16x16/FB_MoveL.FB_MoveL")
    (`self.K2_SetActorLocation` (+ (`self.K2_GetActorLocation`) (-2.0 0.0 0.0)))))

(event `EnhancedInput|/Game/Input/IA_MoveRight`
  (params (ActionValue :type Boolean) (ElapsedSeconds :type "Float (double-precision)") (TriggeredSeconds :type "Float (double-precision)") (InputAction :type "InputAction Object Reference" :default "/Game/Input/IA_MoveRight.IA_MoveRight"))
  (:`Triggered`
    (`PaperFlipbookComponent.SetFlipbook` (`self.Sprite`) "/Game/Assets/PlayerTextures/16x16/FB_MoveR.FB_MoveR")
    (`self.K2_SetActorLocation` (+ (`self.K2_GetActorLocation`) (2.0 0.0 0.0)))))

(event `EnhancedInput|/Game/Input/IA_MoveUp`
  (params (ActionValue :type Boolean) (ElapsedSeconds :type "Float (double-precision)") (TriggeredSeconds :type "Float (double-precision)") (InputAction :type "InputAction Object Reference" :default "/Game/Input/IA_MoveUp.IA_MoveUp"))
  (:`Triggered`
    (`PaperFlipbookComponent.SetFlipbook` (`self.Sprite`) "/Game/Assets/PlayerTextures/16x16/FB_MoveU.FB_MoveU")
    (`self.K2_SetActorLocation` (+ (`self.K2_GetActorLocation`) (0.0 0.0 2.0)))))

(event `self.ReceiveTick`
  (params (DeltaSeconds :type "Float (single-precision)"))
  (bind _returnvalue (`self.K2_GetActorLocation`))
  (bind _outhit (`KismetSystemLibrary.SphereTraceSingle` _returnvalue (+ _returnvalue (* (`self.GetActorForwardVector`) (10.0 10.0 10.0))) 0.0 "TraceTypeQuery3"))
  (`KismetSystemLibrary.PrintString` (`KismetSystemLibrary.GetDisplayName` (`.HitActor` (`GameplayStatics.BreakHitResult` _outhit)))))

(fn `UserConstructionScript`)