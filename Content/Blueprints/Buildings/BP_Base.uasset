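; Building base Blueprint with two functions that raise random popup events for the player.
; Each rerolls against event Chance until one passes, then idles the player sprite and fills a widget, calling Random separately per field, so fields can mix events.
; Random1ButtonEvent applies stat modifiers, shows the popup and pauses the game.
; Random2ButtonEvent sets Yes/No text but never exits its loop, leaving display and pause unreachable.
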(event `self.ReceiveBeginPlay`)

(fn `Random1ButtonEvent`
  (params (Events :type "Array of /Game/Structures/S_1ButtonEvent Structure"))
  (bind _outitem (`KismetArrayLibrary.Array_Random` Events))
  (bind _returnvalue (`PlayerState.GetPlayerController` (`GameplayStatics.GetPlayerState` 0)))
  (bind _returnvalue_2 (`|CreateWidget` "/Game/Widgets/W_General/W_1Butt.W_1Butt_C" _returnvalue))
  (while true
    (if (< (`KismetMathLibrary.RandomFloatInRange` 0.0 100.0) (`.Chance_20_6FD1DFA54C0ADA98177858AAF62FFC27` (break `/Game/Structures/S_1ButtonEvent` _outitem)))
      (bind _asbp_player (cast `/Game/Blueprints/Player/BP_Player` (`GameplayStatics.GetPlayerCharacter` 0)))
      (`PaperFlipbookComponent.SetFlipbook` (`PaperCharacter.Sprite` _asbp_player) "/Game/Assets/PlayerTextures/16x16/FB_IdleD.FB_IdleD")
      (`TextBlock.SetText` (`/Game/Widgets/W_General/W_1Butt.PromptText` _returnvalue_2) (`KismetTextLibrary.Conv_StringToText` (break `/Game/Structures/S_1ButtonEvent` _outitem)))
      (`TextBlock.SetText` (`/Game/Widgets/W_General/W_1Butt.ButtText` _returnvalue_2) (`KismetTextLibrary.Conv_StringToText` (`.ButtonText_4_A727C9D2482E04C9477D12A5B2934CCC` (break `/Game/Structures/S_1ButtonEvent` _outitem))))
      (set `/Game/Blueprints/Player/BP_Player.Health` (+ (`/Game/Blueprints/Player/BP_Player.Health` _asbp_player) (`.HealthModifier_24_555FE00F4C3EAE3327D0E689C1DCA685` (break `/Game/Structures/S_1ButtonEvent` _outitem))) _asbp_player)
      (set `/Game/Blueprints/Player/BP_Player.Money` (+ (`/Game/Blueprints/Player/BP_Player.Money` _asbp_player) (`.MoneyModifier_25_CD8E26FA4B215FB076CEC7B1CB3D5AAE` (break `/Game/Structures/S_1ButtonEvent` _outitem))) _asbp_player)
      (set `/Game/Blueprints/Player/BP_Player.Happiness` (+ (`/Game/Blueprints/Player/BP_Player.Happiness` _asbp_player) (`.HappinessModifier_26_54D4F82C406A7FFA223E648D44AFF2C0` (break `/Game/Structures/S_1ButtonEvent` _outitem))) _asbp_player)
      (set `/Game/Blueprints/Player/BP_Player.Knowledge` (+ (`/Game/Blueprints/Player/BP_Player.Knowledge` _asbp_player) (`.KnowledgeModifier_27_CD857F434F2D2BE4873830B0DB3AF49D` (break `/Game/Structures/S_1ButtonEvent` _outitem))) _asbp_player)
      (set `/Game/Blueprints/Player/BP_Player.HoursLeft` (+ (`/Game/Blueprints/Player/BP_Player.HoursLeft` _asbp_player) (`.HoursLeftModifier_30_03C77AE346006FB824A05ABE4052AEA2` (break `/Game/Structures/S_1ButtonEvent` _outitem))) _asbp_player)
      (`UserWidget.AddToViewport` _returnvalue_2 0)
      (set `PlayerController.bShowMouseCursor` true _returnvalue)
      (`GameplayStatics.SetGamePaused` true)
      (return))))

(fn `Random2ButtonEvent`
  (params (Events :type "Array of /Game/Structures/S_2ButtonsEvent Structure"))
  (bind _outitem (`KismetArrayLibrary.Array_Random` Events))
  (bind _returnvalue (`|CreateWidget` "/Game/Widgets/W_General/W_2Butt.W_2Butt_C" (`PlayerState.GetPlayerController` (`GameplayStatics.GetPlayerState` 0))))
  (while true
    (if (< (`KismetMathLibrary.RandomFloatInRange` 0.0 100.0) (`.Chance_23_7D0FF0294F13707EE219D891E21EF8F5` (break `/Game/Structures/S_2ButtonsEvent` _outitem)))
      (bind _asbp_player (cast `/Game/Blueprints/Player/BP_Player` (`GameplayStatics.GetPlayerCharacter` 0)))
      (`PaperFlipbookComponent.SetFlipbook` (`PaperCharacter.Sprite` _asbp_player) "/Game/Assets/PlayerTextures/16x16/FB_IdleD.FB_IdleD")
      (`TextBlock.SetText` (`/Game/Widgets/W_General/W_2Butt.PromptText` _returnvalue) (`KismetTextLibrary.Conv_StringToText` (break `/Game/Structures/S_2ButtonsEvent` _outitem)))
      (`TextBlock.SetText` (`/Game/Widgets/W_General/W_2Butt.ButtTextYES` _returnvalue) (`KismetTextLibrary.Conv_StringToText` (`.ButtonYESText_26_E8B058ED4E8F6054D218E4AB172B1ECF` (break `/Game/Structures/S_2ButtonsEvent` _outitem))))
      (`TextBlock.SetText` (`/Game/Widgets/W_General/W_2Butt.ButtTextNO` _returnvalue) (`KismetTextLibrary.Conv_StringToText` (`.ButtonNOText_27_90426A0E4F096FEF9CB1C98A0F07D644` (break `/Game/Structures/S_2ButtonsEvent` _outitem)))))))

(fn `UserConstructionScript`)