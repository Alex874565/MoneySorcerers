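; BP_Funkytown is a building Blueprint that opens the W_FunkyTown screen through its ShowWidget event.
; The event casts the player character to BP_Player and switches its sprite to the FB_IdleD idle flipbook.
; It then shows the mouse cursor, pauses the game and adds a newly created widget to the viewport.
; Nothing in this Blueprint calls ShowWidget or handles closing and unpausing.
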(event `/Game/Blueprints/Interfaces/BPI_ShowWidget.ShowWidget`
  (bind _asbp_player (cast `/Game/Blueprints/Player/BP_Player` (`GameplayStatics.GetPlayerCharacter` 0)))
  (`PaperFlipbookComponent.SetFlipbook` (`PaperCharacter.Sprite` _asbp_player) "/Game/Assets/PlayerTextures/16x16/FB_IdleD.FB_IdleD")
  (set `PlayerController.bShowMouseCursor` true (`GameplayStatics.GetPlayerController` 0))
  (`GameplayStatics.SetGamePaused` true)
  (bind _returnvalue (`|CreateWidget` "/Game/Widgets/W_General/W_FunkyTown.W_FunkyTown_C"))
  (`UserWidget.AddToViewport` _returnvalue 0))

(fn `UserConstructionScript`
  (`parent.UserConstructionScript`))